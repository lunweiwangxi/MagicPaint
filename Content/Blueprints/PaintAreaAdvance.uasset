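; PaintAreaAdvance extends the PaintAreaBase touch painting area with particle effects that follow each touch.
; BeginPlay pre-spawns a pool of ten inactive emitters, one per supported touch point, indexed by TouchIndex.
; Painting runs the parent logic, then activates and moves that touch's emitter just above the hit point, except in one paint mode.
; UnPainting runs the parent stop logic and deactivates the emitter.
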(event `self.ReceiveBeginPlay`
  (`parent.ReceiveBeginPlay`)
  ;[1 1 1] 生成10个粒子(触摸屏支持10个点的触碰)
  (for _ (range 10)
    (bind _returnvalue (`GameplayStatics.SpawnEmitterAtLocation` (`self.FollowPSTemplate`) (0.0 0.0 0.0) (struct) (1.0 1.0 1.0) false))
    (`ActorComponent.SetActive` _returnvalue false false)
    (`KismetArrayLibrary.Array_Add` (`self.FollowPSs`) _returnvalue)))

(event `self.Painting`
  (params (TouchIndex :type Integer) (uvPos :type "Vector2D Structure") (hitPos :type "Vector Structure"))
  (bind _output (`|GetArrayItem` (`self.FollowPSs`) TouchIndex))
  ;[1 1 1] 绘制逻辑,详见PaintAreaBase::Painting
  ; Paint Logic,More in PaintAreaBase::Painting
  (`parent.Painting` TouchIndex uvPos hitPos)
  ;[1 1 1] 触摸滑动,让对应的粒子运作
  ; TouchMove,Activate the corresponding particle
  (if (`|EnumInequality` (`self.PaintMode`) "NewEnumerator2")
    (`ActorComponent.SetActive` _output true false)
    (`SceneComponent.K2_SetWorldLocation` _output (+ hitPos (0.0 0.0 10.0)) true false)))

(event `self.UnPainting`
  (params (TouchIndex :type Integer))
  ;[1 1 1] 停止绘制逻辑,详见PaintAreaBase::UnPainting
  ; Stop paint Logic,More in PaintAreaBase:UnPainting
  (`parent.UnPainting` TouchIndex)
  ;[1 1 1] 触摸松开,让对应的粒子失活
  ; TouchEnd,Deactivate the corresponding particle
  (`ActorComponent.SetActive` (`|GetArrayItem` (`self.FollowPSs`) TouchIndex) false false))

(fn `UserConstructionScript`
  (`parent.UserConstructionScript`))