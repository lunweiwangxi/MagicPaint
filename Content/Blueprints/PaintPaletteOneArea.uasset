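; Paint palette actor that manages a single drawable paint area and its on-screen UI.
; On BeginPlay it adds a UI_DrawAreaOneArea widget to the viewport, passing itself as owner, and caches the PaintAreaBase from the PaintAreaAdvanceCmp child actor.
; Its functions forward paint mode, color and size changes to that area, switching on an area-position enum that handles only Area 1.
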(event `self.ReceiveBeginPlay`
  (`|ExecutionSequence`
    (:`then_0`
      (bind _returnvalue (`|CreateWidget` "/MagicPainting/Widgets/UI_DrawAreaOneArea.UI_DrawAreaOneArea_C" null self))
      (bind _output_get (set `self.UI` _returnvalue))
      (`UserWidget.AddToViewport` _output_get 0))
    (:`then_1`
      (bind _aspaint_area_base (cast `/MagicPainting/Blueprints/PaintAreaBase` (`ChildActorComponent.ChildActor` (`self.PaintAreaAdvanceCmp`))))
      (set `self.PaintAreaBase` _aspaint_area_base))))

(fn `OnPaintSizeChange`
  (params (PaintAreaPos :type "/MagicPainting/Blueprints/PaintAreaPostion Enum" :default "NewEnumerator0") (Value :type "Float (double-precision)"))
  (switch `/MagicPainting/Blueprints/PaintAreaPostion` PaintAreaPos
    (:`NewEnumerator0`
      (`/MagicPainting/Blueprints/PaintAreaBase.OnPaintSizeChange` (`self.PaintAreaBase`) (`local.Value`)))))

(fn `SetPaintColorByIndex`
  (params (PaintAreaPos :type "/MagicPainting/Blueprints/PaintAreaPostion Enum" :default "NewEnumerator0") (LColor :type "LinearColor Structure"))
  (switch `/MagicPainting/Blueprints/PaintAreaPostion` PaintAreaPos
    (:`NewEnumerator0`
      (`/MagicPainting/Blueprints/PaintAreaBase.OnPaintColorChange` (`self.PaintAreaBase`) (`local.LColor`)))))

(fn `SetPaintModeByIndex`
  (params (PaintAreaPos :type "/MagicPainting/Blueprints/PaintAreaPostion Enum" :default "NewEnumerator0") (PaintMode :type "/MagicPainting/Blueprints/PaintMode Enum" :default "NewEnumerator0"))
  (switch `/MagicPainting/Blueprints/PaintAreaPostion` PaintAreaPos
    (:`NewEnumerator0`
      (`/MagicPainting/Blueprints/PaintAreaBase.OnPaintModeChange` (`self.PaintAreaBase`) (`local.PaintMode`)))))

(fn `UserConstructionScript`)