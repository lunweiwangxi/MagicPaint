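; Base paint-board actor that lets the player draw on a surface with pen, brush or eraser.
; On BeginPlay it creates and clears a render target, feeds it to the board's dynamic material, and creates a dynamic material for each tool.
; Painting stamps the active tool's material onto the render target via canvas draw, centered on the given UV.
; Change handlers switch tool, recolor pen and brush, and set stamp size.
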(event `self.ReceiveBeginPlay`
  (bind (_paintboardres_x _paintboardres_y) (`KismetMathLibrary.BreakVector2D` (`self.PaintBoardRes`)))
  (`|ExecutionSequence`
    (:`then_0`
      (bind _returnvalue (`KismetRenderingLibrary.CreateRenderTarget2D` (`KismetMathLibrary.FTrunc` _paintboardres_x) (`KismetMathLibrary.FTrunc` _paintboardres_y) "RTF_RGB10A2")) ; 创建RT2D
      (bind _output_get (set `self.PaintBoardRT2D` _returnvalue))
      (`KismetRenderingLibrary.ClearRenderTarget2D` _output_get)
      (bind _returnvalue_2 (`KismetMaterialLibrary.CreateDynamicMaterialInstance` (`self.PaintBoardMat`))) ; DM_绘画区域
      (set `self.PaintBoardMatDM` _returnvalue_2)
      (`MaterialInstanceDynamic.SetTextureParameterValue` (`self.PaintBoardMatDM`) "RenderTarget" (`self.PaintBoardRT2D`)) ; DrawRT给DrawMatDM
      (`PrimitiveComponent.SetMaterial` (`self.DrawAreaCmp`) 0 (`self.PaintBoardMatDM`)))
    (:`then_1`
      (bind _returnvalue_3 (`KismetMaterialLibrary.CreateDynamicMaterialInstance` (`self.PenMat`))) ; DM_画笔
      (set `self.PenMatDM` _returnvalue_3)
      (`MaterialInstanceDynamic.SetVectorParameterValue` (`self.PenMatDM`) "PaintColor" (`self.PaintColor`)) ; 初始化Pen颜色
      (set `self.CurUseMaterial` (`self.PenMatDM`)) ; 默认画笔为Pen
    )
    (:`then_2`
      (bind _returnvalue_4 (`KismetMaterialLibrary.CreateDynamicMaterialInstance` (`self.BrushMat`))) ; DM_画刷
      (set `self.BrushMatDM` _returnvalue_4)
      (`MaterialInstanceDynamic.SetVectorParameterValue` (`self.BrushMatDM`) "PaintColor" (`self.PaintColor`)) ; 初始化Brush颜色
    )
    (:`then_3`
      (bind _returnvalue_5 (`KismetMaterialLibrary.CreateDynamicMaterialInstance` (`self.EraserMat`))) ; DM_橡皮擦
      (set `self.EraserMatDM` _returnvalue_5)
      (`MaterialInstanceDynamic.SetVectorParameterValue` (`self.EraserMatDM`) "PaintColor" (`self.EraserColor`)) ; 初始化Eraser颜色
    )))

(fn `OnPaintColorChange`
  (params (LColor :type "LinearColor Structure"))
  (set `self.PaintColor` LColor)
  (`MaterialInstanceDynamic.SetVectorParameterValue` (`self.PenMatDM`) "PaintColor" (`self.PaintColor`))
  (`MaterialInstanceDynamic.SetVectorParameterValue` (`self.BrushMatDM`) "PaintColor" (`self.PaintColor`)))

(fn `OnPaintModeChange`
  (params (PaintMode :type "/MagicPainting/Blueprints/PaintMode Enum" :default "NewEnumerator0"))
  (bind _output_get (set `self.PaintMode` PaintMode))
  (switch `/MagicPainting/Blueprints/PaintMode` _output_get
    (:`NewEnumerator0`
      (set `self.CurUseMaterial` (`self.PenMatDM`)))
    (:`NewEnumerator1`
      (set `self.CurUseMaterial` (`self.BrushMatDM`)))
    (:`NewEnumerator2`
      (set `self.CurUseMaterial` (`self.EraserMatDM`)))))

(fn `OnPaintSizeChange`
  (params (Value :type "Float (double-precision)"))
  (set `self.PaintSize` (+ (80.0 80.0) (* Value 200.0))))

(fn `Painting`
  (params (TouchIndex :type Integer) (uvPos :type "Vector2D Structure") (hitPos :type "Vector Structure"))
  (bind (_canvas _size _context) (`KismetRenderingLibrary.BeginDrawCanvasToRenderTarget` (`self.PaintBoardRT2D`)))
  (`Canvas.K2_DrawMaterial` _canvas (`self.CurUseMaterial`) (- (* _size (`local.uvPos`)) (/ (`self.PaintSize`) 2.0)) (`self.PaintSize`) (0.0 0.0) (1.0 1.0) 0.0 (0.5 0.5))
  (`KismetRenderingLibrary.EndDrawCanvasToRenderTarget` _context))

(fn `PaintSizeChange`
  (params (size :type "Vector2D Structure"))
  (set `self.PaintSize` size))

(fn `UnPainting`
  (params (TouchIndex :type Integer)))

(fn `UserConstructionScript`)