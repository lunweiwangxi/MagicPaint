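; PaintPaletteTwoArea is a paint palette actor that manages two paint areas, left and mid, with an on-screen UI.
; On BeginPlay it creates the UI_DrawAreaTwoArea widget with a reference to itself and caches both child actors as PaintAreaBase.
; Its mode, color and size functions switch on an area position and forward the change to the matching area.
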(event `self.ReceiveBeginPlay`
  (`|ExecutionSequence`
    (:`then_0`
      (bind _returnvalue (`|CreateWidget` "/MagicPainting/Widgets/UI_DrawAreaTwoArea.UI_DrawAreaTwoArea_C" null self))
      (bind _output_get (set `self.UI` _returnvalue))
      (`UserWidget.AddToViewport` _output_get 0))
    (:`then_1`
      (bind _aspaint_area_base (cast `/MagicPainting/Blueprints/PaintAreaBase` (`ChildActorComponent.ChildActor` (`self.PaintAreaAdvanceCmpLeft`))))
      (set `self.PaintAreaLeft` _aspaint_area_base))
    (:`then_2`
      (bind _aspaint_area_base_2 (cast `/MagicPainting/Blueprints/PaintAreaBase` (`ChildActorComponent.ChildActor` (`self.PaintAreaAdvanceCmpMid`))))
      (set `self.PaintAreaMid` _aspaint_area_base_2))))

(fn `OnPaintSizeChange`
  (params (PaintAreaPos :type "/MagicPainting/Blueprints/PaintAreaPostion Enum" :default "NewEnumerator0") (Value :type "Float (double-precision)"))
  (switch `/MagicPainting/Blueprints/PaintAreaPostion` PaintAreaPos
    (:`NewEnumerator0`
      (`/MagicPainting/Blueprints/PaintAreaBase.OnPaintSizeChange` (`self.PaintAreaLeft`) (`local.Value`)))
    (:`NewEnumerator1`
      (`/MagicPainting/Blueprints/PaintAreaBase.OnPaintSizeChange` (`self.PaintAreaMid`) (`local.Value`)))))

(fn `SetPaintColorByIndex`
  (params (PaintAreaPos :type "/MagicPainting/Blueprints/PaintAreaPostion Enum" :default "NewEnumerator0") (LColor :type "LinearColor Structure"))
  (switch `/MagicPainting/Blueprints/PaintAreaPostion` PaintAreaPos
    (:`NewEnumerator0`
      (`/MagicPainting/Blueprints/PaintAreaBase.OnPaintColorChange` (`self.PaintAreaLeft`) (`local.LColor`)))
    (:`NewEnumerator1`
      (`/MagicPainting/Blueprints/PaintAreaBase.OnPaintColorChange` (`self.PaintAreaMid`) (`local.LColor`)))))

(fn `SetPaintModeByIndex`
  (params (PaintAreaPos :type "/MagicPainting/Blueprints/PaintAreaPostion Enum" :default "NewEnumerator0") (PaintMode :type "/MagicPainting/Blueprints/PaintMode Enum" :default "NewEnumerator0"))
  (switch `/MagicPainting/Blueprints/PaintAreaPostion` PaintAreaPos
    (:`NewEnumerator0`
      (`/MagicPainting/Blueprints/PaintAreaBase.OnPaintModeChange` (`self.PaintAreaLeft`) (`local.PaintMode`)))
    (:`NewEnumerator1`
      (`/MagicPainting/Blueprints/PaintAreaBase.OnPaintModeChange` (`self.PaintAreaMid`) (`local.PaintMode`)))))

(fn `UserConstructionScript`)