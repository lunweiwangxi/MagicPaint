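; Pawn that lets the player paint on PaintAreaAdvance actors by dragging with the left mouse button.
; While held, MouseX movement line-traces from the cursor and passes hit UV and impact point to Painting.
; Releasing calls UnPainting on every PaintAreaBase.
; UV lookup requires the Support UV From Hit Results project setting; per-finger touch logic targeting PaintAreaBase is present but unconnected.
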(event `self.ReceiveBeginPlay`
  (set `PlayerController.bShowMouseCursor` true (`GameplayStatics.GetPlayerController` 0)))

(event `Key|LeftMouseButton`
  (params (Key :type "Key Structure"))
  ;[1 1 1] 鼠标测试代码,在触摸屏上禁用这些代码
  (:`Pressed`
    (set `self.LeftMousePress` true))
  (:`Released`
    (set `self.LeftMousePress` false)
    (bind _outactors (`GameplayStatics.GetAllActorsOfClass` "/MagicPainting/Blueprints/PaintAreaBase.PaintAreaBase_C"))
    (for _array_element _outactors
      (`/MagicPainting/Blueprints/PaintAreaBase.UnPainting` _array_element 0))))

(event `InputAxisKey|MouseX`
  (params (AxisValue :type "Float (single-precision)"))
  (bind (_worldlocation _worlddirection) (`PlayerController.DeprojectMousePositionToWorld` (`GameplayStatics.GetPlayerController` 0)))
  ;[1 1 1] 鼠标测试代码,在触摸屏上禁用这些代码
  (if (and (!= AxisValue 0.0) (`self.LeftMousePress`))
    (bind (_outhit _returnvalue) (`KismetSystemLibrary.LineTraceSingle` _worldlocation (+ _worldlocation (* _worlddirection 10000.0)) "TraceTypeQuery1" true))
    (if _returnvalue
      (bind (_bblockinghit _binitialoverlap _time _distance _location _impactpoint _normal _impactnormal _physmat _hitactor) (`GameplayStatics.BreakHitResult` _outhit))
      (bind _aspaint_area_advance (cast `/MagicPainting/Blueprints/PaintAreaAdvance` _hitactor))
      (bind (_uv _returnvalue_2) (`GameplayStatics.FindCollisionUV` _outhit))
      (if _returnvalue_2
        (`/MagicPainting/Blueprints/PaintAreaBase.Painting` _aspaint_area_advance 0 _uv _impactpoint)))))

(event `InputTouch`
  (params (Location :type "Vector Structure") (FingerIndex :type "ETouchIndex Enum"))
  ;[1 1 1] 触摸屏事件
)

(event `InputTouch`
  (params (Location :type "Vector Structure") (FingerIndex :type "ETouchIndex Enum"))
  ;[1 1 1] 触摸屏事件
)

(fn `UserConstructionScript`)